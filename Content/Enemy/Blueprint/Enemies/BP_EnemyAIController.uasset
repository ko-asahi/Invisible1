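; Enemy AI controller that stages brawl animations when a pending AI interaction starts.
; When the behavior tag matches Behavior.AI.Interact.Brawl, it plays a brawl montage on its controlled character.
; If the target actor is another BP_EnemyTest, it also has that enemy play the paired hit montage through PlayBrawlHitMontage.
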(event `self.BP_OnPendingInteractionStarted`
  (params (TargetActor :type "Actor Object Reference") (BehaviorTag :type "GameplayTag Structure") (Duration :type "Float (single-precision)"))
  (bind _returnvalue (`self.K2_GetPawn`))
  (if (`BlueprintGameplayTagLibrary.MatchesTag` BehaviorTag (struct :`TagName` "Behavior.AI.Interact.Brawl"))
    (`/Engine/EditorBlueprintResources/StandardMacros.IsValid` _returnvalue
      (:`Is Valid`
        (bind `_as角色` (cast `Character` _returnvalue))
        (`Character.PlayAnimMontage` `_as角色` "/Game/Animation/Animation/EnemyAni/PROJ2小兵-打斗动画1_Montage.PROJ2小兵-打斗动画1_Montage" 1.0 "None")
        (`/Engine/EditorBlueprintResources/StandardMacros.IsValid` TargetActor
          (:`Is Valid`
            (if (!= _returnvalue TargetActor)
              (bind _asbp_enemy_test (cast `/Game/Enemy/Blueprint/Enemies/BP_EnemyTest` TargetActor))
              (`/Game/Enemy/Blueprint/Enemies/BP_EnemyTest.PlayBrawlHitMontage` _asbp_enemy_test "/Game/Animation/Animation/EnemyAni/PROJ2小兵-打斗动画2_Montage.PROJ2小兵-打斗动画2_Montage"))))))))

(fn `UserConstructionScript`)