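; Spline-driven path actor that draws a procedural mesh line with optional start and end planes, such as arrowheads.
; The construction script samples the spline by segment length, trims the ends to fit the planes, builds vertices, triangles and UVs, and centers a billboard above the path.
; Helper events flatten or recenter the spline, requiring a manual construction refresh to update the visuals.
; Route-provider functions return only empty defaults.
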(event `Align Spline Horizontal`
  ;[1 0 0.1564 0.1 14] This Event aligns all spline points in the horizontal plane.
  ; Due to the way the construction script works, the visual path will not be updated,
  ; you need to click on the Update parameter or move the entire spline or actor.
  (for _index (range (`SplineComponent.GetNumberOfSplinePoints` (`self.Spline`)))
    (`SplineComponent.SetLocationAtSplinePoint` (`self.Spline`) _index (`KismetMathLibrary.MakeVector` (.x (`SplineComponent.GetLocationAtSplinePoint` (`self.Spline`) _index "Local")) (.y (`SplineComponent.GetLocationAtSplinePoint` (`self.Spline`) _index "Local"))) "Local" false))
  (`SplineComponent.UpdateSpline` (`self.Spline`)))

(event `Offset Spline Points To Actor Center`
  ;[1 0 0.1564 0.1 14] This Event aligns the center of the actor to the center of the spline,
  ; useful if you have moved the spline points too far and the actor becomes awkward to move or rotate.
  ; Due to the way the construction script works, the visual path will not be updated,
  ; you need to click on the Update parameter or move the spline or the entire actor, after which you need to reselect the actor to update the movement gizmo.
  (bind _splinepoints (`self.GetSplinePoints` true))
  (set `self.ActorCenter` (`KismetMathLibrary.GetVectorArrayAverage` _splinepoints))
  (`self.OffsetSplinePoints` (`self.ActorCenter`))
  (`self.K2_SetActorLocation` (+ (`self.K2_GetActorLocation`) (`self.ActorCenter`))))

(fn `DrawPath`
  (params (PathPoints :type "Array of Vector Structure"))
  (locals (SplinePointsLOCAL :type "Array of Vector Structure") (TrimSplinePointsLOCAL :type "Array of Vector Structure") (EndPointLOCAL :type "Vector Structure"))
  (bind _returnvalue (/ (`self.StartPlaneSize`) 100.0))
  (bind _returnvalue_2 (/ (`self.EndPlaneSize`) 100.0))
  (set `local.SplinePointsLOCAL` PathPoints)
  (`|ExecutionSequence`
    (:`then_0`
      (if (or (`self.EnableStartPlane`) (`self.EnableEndPlane`))
        ;[1 0 0.1564 0.1 14] Path ends may not be displayed correctly if there are other points very close to them.
        ; This function will remove points that are close to both ends of the path.
        ; (In the Arrow example, this function allows the end of the arrow to always point exactly to the last point on the path)
        (bind _returnvalue_3 (`self.RemoveSmallSegmentsCloseToBothEnds` (`local.SplinePointsLOCAL`) (`self.EnableStartPlane`) (`self.StartPlaneSize`) (`self.EnableEndPlane`) (`self.EndPlaneSize`)))
        (set `local.SplinePointsLOCAL` _returnvalue_3)
        ;[1 0 0.1564 0.1 14] This logic is responsible for the correct position and rotation of the start and end planes.
        ; The Trim Path Complex function trims the path depending on the location and size of the start and end planes.
        (set `self.StartPlaneOffset` (`KismetMathLibrary.FClamp` (`self.StartPlaneOffset`)))
        (set `self.EndPlaneOffset` (`KismetMathLibrary.FClamp` (`self.EndPlaneOffset`)))
        (bind (_trimpoints _starttrimpoint _startrotation _startdirection _endtrimpoint _endrotation) (`self.TrimPathComplex` (`local.SplinePointsLOCAL`) (`self.EnableStartPlane`) (* (`self.StartPlaneSize`) (`self.StartPlaneOffset`)) (`self.EnableEndPlane`) (* (`self.EndPlaneSize`) (`self.EndPlaneOffset`))))
        (set `local.TrimSplinePointsLOCAL` _trimpoints)
        (`|ExecutionSequence`
          (:`then_0`
            (if (`self.EnableStartPlane`)
              (`SceneComponent.K2_SetRelativeTransform` (`self.StartPlane`) (`KismetMathLibrary.MakeTransform` _starttrimpoint _startrotation (`KismetMathLibrary.MakeVector` _returnvalue _returnvalue 1.0)) false false)))
          (:`then_1`
            (if (`self.EnableEndPlane`)
              (`SceneComponent.K2_SetRelativeTransform` (`self.EndPlane`) (`KismetMathLibrary.MakeTransform` _endtrimpoint _endrotation (`KismetMathLibrary.MakeVector` _returnvalue_2 _returnvalue_2 1.0)) false false))))
        (else
          (set `local.TrimSplinePointsLOCAL` (`local.SplinePointsLOCAL`)))))
    (:`then_1`
      ;[1 0 0.1564 0.1 14] This function calculates all vertices, triangles and UVs, depending on the settings.
      ; This data is needed to draw polygons along a path using a procedural mesh.
      (bind (_vertexes _triangles _uv _returnvalue_4) (`self.GetPathData` (`local.TrimSplinePointsLOCAL`) false (`self.Thickness`) 0.0 (`self.EnableUV`) (`self.ScaleUV`) (`self.OffsetUV`)))
      ;[1 0 0.1564 0.1 14] Creates a mesh.
      (if _returnvalue_4
        (`ProceduralMeshComponent.CreateMeshSection_LinearColor` :`self` (`self.ProceduralMesh`) :`Vertices` _vertexes :`Triangles` _triangles :`UV0` _uv)))))

(fn `GetProviderBehaviorAnchorYawForRoutePoint`
  (params (RoutePointWorldLocation :type "Vector Structure (by ref)"))
  (returns (OutYaw :type "Float (single-precision)") (ReturnValue :type Boolean))
  (return 0.0 false))

(fn `GetProviderBehaviorDataForRoutePoint`
  (params (RoutePointWorldLocation :type "Vector Structure (by ref)"))
  (returns (OutBehavior :type "EWaypointBehavior Enum") (OutWaitTime :type "Float (single-precision)") (OutLookAngle :type "Float (single-precision)") (OutLookSpeed :type "Float (single-precision)") (bOutUseCustomLookCenter :type Boolean) (OutLookCenterYawOffset :type "Float (single-precision)") (OutPreLookPauseTime :type "Float (single-precision)"))
  (return "None" 0.0 0.0 0.0 false 0.0 0.0))

(fn `GetProviderRoutePoint`
  (params (Index :type Integer))
  (returns (OutPoint :type "Vector Structure") (ReturnValue :type Boolean))
  (return (0.0 0.0 0.0) false))

(fn `GetProviderRoutePointCount`
  (returns (ReturnValue :type Integer))
  (return 0))

(fn `GetProviderRoutePoints`
  (returns (OutPoints :type "Array of Vector Structure"))
  (return))

(fn `GetSplinePoints`
  (params (`2D` :type Boolean))
  (returns (SplinePoints :type "Array of Vector Structure"))
  (locals (SplinePointsLOCAL :type "Array of Vector Structure") (IterationsLOCAL :type Integer :default 0) (`2DLOCAL` :type Boolean) (LastPointLOCAL :type "Vector Structure"))
  (bind _lastpointlocal (`local.LastPointLOCAL`))
  (bind _spline (`self.Spline`))
  (bind _segmentlength (`self.SegmentLength`))
  (bind _returnvalue (`SplineComponent.GetLocationAtSplinePoint` (`self.Spline`) 0 "Local"))
  (bind _returnvalue_2 (`SplineComponent.GetLocationAtSplinePoint` _spline (- (`SplineComponent.GetNumberOfSplinePoints` _spline) 1) "Local"))
  (set `local.2DLOCAL` `2D`)
  (set `self.SegmentLength` (`KismetMathLibrary.FClamp` _segmentlength 1.0 _segmentlength))
  (if (!= (`SplineComponent.GetNumberOfSplinePoints` (`self.Spline`)) 1)
    (set `local.IterationsLOCAL` (`.ReturnValue` (`KismetMathLibrary.FMod` (`SplineComponent.GetSplineLength` (`self.Spline`)) (`self.SegmentLength`))))
    (`|ExecutionSequence`
      (:`then_0`
        (set `local.LastPointLOCAL` (`SplineComponent.GetLocationAtSplinePoint` (`self.Spline`) 0 "Local"))
        (if (`local.2DLOCAL`)
          (`KismetArrayLibrary.Array_Add` (`local.SplinePointsLOCAL`) (`KismetMathLibrary.MakeVector` (.x _lastpointlocal) (.y _lastpointlocal)))
          (else
            (`KismetArrayLibrary.Array_Add` (`local.SplinePointsLOCAL`) _lastpointlocal))))
      (:`then_1`
        (for _index (range 1 (`local.IterationsLOCAL`))
          (if (`local.2DLOCAL`)
            (bind _returnvalue_3 (`SplineComponent.GetLocationAtDistanceAlongSpline` (`self.Spline`) (* _index (`self.SegmentLength`)) "Local"))
            (`KismetArrayLibrary.Array_Add` (`local.SplinePointsLOCAL`) (`KismetMathLibrary.MakeVector` (.x _returnvalue_3) (.y _returnvalue_3)))
            (else
              (`KismetArrayLibrary.Array_Add` (`local.SplinePointsLOCAL`) _returnvalue_3))))
        (if (`local.2DLOCAL`)
          (`KismetArrayLibrary.Array_Add` (`local.SplinePointsLOCAL`) (`KismetMathLibrary.MakeVector` (.x _returnvalue_2) (.y _returnvalue_2)))
          (else
            (`KismetArrayLibrary.Array_Add` (`local.SplinePointsLOCAL`) _returnvalue_2))))
      (:`then_2`
        (return (`local.SplinePointsLOCAL`))))
    (else
      (`|ExecutionSequence`
        (:`then_0`
          (if (`local.2DLOCAL`)
            (`KismetArrayLibrary.Array_Add` (`local.SplinePointsLOCAL`) (`KismetMathLibrary.MakeVector` (.x _returnvalue) (.y _returnvalue)))
            (else
              (`KismetArrayLibrary.Array_Add` (`local.SplinePointsLOCAL`) _returnvalue))))
        (:`then_1`
          (return (`local.SplinePointsLOCAL`)))))))

(fn `IsProviderClosedLoop`
  (returns (ReturnValue :type Boolean))
  (return false))

(fn `OffsetSplinePoints`
  (params (Offset :type "Vector Structure"))
  (for _index (range (`SplineComponent.GetNumberOfSplinePoints` (`self.Spline`)))
    (`SplineComponent.SetLocationAtSplinePoint` (`self.Spline`) _index (- (`SplineComponent.GetLocationAtSplinePoint` (`self.Spline`) _index "Local") Offset) "Local" false))
  (`SplineComponent.UpdateSpline` (`self.Spline`)))

(fn `SetActorMaterials`
  (`PrimitiveComponent.SetMaterial` (`self.ProceduralMesh`) 0 (`self.LineMaterial`))
  (`|ExecutionSequence`
    (:`then_0`
      (if (`self.EnableStartPlane`)
        (`PrimitiveComponent.SetMaterial` (`self.StartPlane`) 0 (`self.StartMaterial`))
        (set `self.StartPlaneSize` (* (`self.Thickness`) 2.0 (`self.StartPlaneScale`)))))
    (:`then_1`
      (if (`self.EnableEndPlane`)
        (`PrimitiveComponent.SetMaterial` (`self.EndPlane`) 0 (`self.EndMaterial`))
        (set `self.EndPlaneSize` (* (`self.Thickness`) 2.0 (`self.EndPlaneScale`)))))
    (:`then_2`
      (`SceneComponent.SetVisibility` (`self.StartPlane`) (`self.EnableStartPlane`) false)
      (`SceneComponent.SetVisibility` (`self.EndPlane`) (`self.EnableEndPlane`) false))))

(fn `UserConstructionScript`
  (bind (_pathcenter_x _pathcenter_y _pathcenter_z) (`KismetMathLibrary.BreakVector` (`self.PathCenter`)))
  ;[1 0 0.1564 0.1 14] Set Actor Materials
  (`self.SetActorMaterials`)
  ;[1 0 0.1564 0.1 14] Finds all Spline Points
  (bind _splinepoints (`self.GetSplinePoints` false))
  ;[1 0 0.1564 0.1 14] Draw Path
  (`self.DrawPath` _splinepoints)
  ;[1 0 0.1564 0.1 14] Cosmetic logic intended only to move the billboard and update the actor in the editor.
  ;
  ; If you need a path that will only be drawn during the game, this logic can be left in the Construction Script, it does not need to be transferred to Tick
  (set `self.PathCenter` (`KismetMathLibrary.GetVectorArrayAverage` _splinepoints)) ; Aligns the billboard to the geometric center of the path points
  (`SceneComponent.K2_SetRelativeLocation` (`self.Billboard`) (`KismetMathLibrary.MakeVector` _pathcenter_x _pathcenter_y (+ _pathcenter_z 200.0)) false false) ; Move Billboard in local coordinates
  (set `self.Update` false) ; This variable is needed simply to cause \na forced update of the construction script in the editor
)