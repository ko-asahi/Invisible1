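; BP_PatrolPathVisualizer is an actor that draws a referenced patrol path as a procedural mesh ribbon.
; Its construction script calls RebuildPathMesh, which converts the target's route points to mesh-local space and feeds them, with loop flag, thickness and offset, into GetPathData.
; Valid results become a mesh section using PathMaterial.
; The event graph holds only disabled events and unconnected leftover nodes.
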(fn `RebuildPathMesh`
  (bind _targetpatrolpath (`self.TargetPatrolPath`))
  (bind _pathmesh (`self.PathMesh`))
  (`/Engine/EditorBlueprintResources/StandardMacros.IsValid` _targetpatrolpath
    (:`Is Valid`
      (`ProceduralMeshComponent.ClearAllMeshSections` _pathmesh)
      (bind (_vertexes _triangles _uv _returnvalue) (`self.GetPathData` (`PatrolPath.GetPatrolRoutePointsLocalToComponent` _targetpatrolpath _pathmesh) (`PatrolPath.IsPatrolClosedLoop` _targetpatrolpath) (`self.Thickness`) (`self.Offset`) false (1.0 1.0) (0.0 0.0)))
      (if (and (> (`KismetArrayLibrary.Array_Length` _vertexes) 0) _returnvalue)
        (`ProceduralMeshComponent.CreateMeshSection_LinearColor` :`self` _pathmesh :`Vertices` _vertexes :`Triangles` _triangles :`UV0` _uv)
        (`PrimitiveComponent.SetMaterial` _pathmesh 0 (`self.PathMaterial`))))))

(fn `UserConstructionScript`
  (`self.RebuildPathMesh`))